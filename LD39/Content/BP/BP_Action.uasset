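; BP_Action is a timed action, apparently for attacks, with a duration phase and a cooldown tracked by two timer handles.
; StartAction starts the duration timer when neither timer has time left, otherwise printing a warning, while ActionFinished starts the cooldown timer.
; Query functions expose remaining times and state, though IsCoolingDown tests the Cooldown value instead of its timer.
; IsInWindow requires remaining time at or below both zero and SuccessWindow.
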(event `self.ReceiveBeginPlay`
  (`KismetSystemLibrary.K2_ClearAndInvalidateTimerHandle` (`self.Timer`))
  (`KismetSystemLibrary.K2_ClearAndInvalidateTimerHandle` (`self.CooldownTimer`)))

(fn `ActionFinished`
  (bind _returnvalue (`KismetSystemLibrary.K2_SetTimerDelegate` (`|CreateDelegate` :!event `CooldownFinished`) (`self.Cooldown`)))
  (set `self.CooldownTimer` _returnvalue))

(fn `CanAttack`
  (returns (`CanAttack?` :type Boolean))
  (return (and (<= (`KismetSystemLibrary.K2_GetTimerRemainingTimeHandle` (`self.CooldownTimer`)) 0.0) (<= (`KismetSystemLibrary.K2_GetTimerRemainingTimeHandle` (`self.Timer`)) 0.0))))

(fn `CooldownFinished`)

(fn `GetCoolDownTime`
  (returns (CooldownRemaining :type "Float (double-precision)"))
  (return (`KismetSystemLibrary.K2_GetTimerRemainingTimeHandle` (`self.CooldownTimer`))))

(fn `GetTime`
  (returns (TimeRemaing :type "Float (double-precision)"))
  (return (`KismetSystemLibrary.K2_GetTimerRemainingTimeHandle` (`self.Timer`))))

(fn `IsActing`
  (returns (`IsActing?` :type Boolean))
  (return (>= (`KismetSystemLibrary.K2_GetTimerRemainingTimeHandle` (`self.Timer`)) 0.0)))

(fn `IsCoolingDown`
  (returns (`CoolingDown?` :type Boolean))
  (return (<= (`self.Cooldown`) 0.0)))

(fn `IsInWindow`
  (returns (`InSuccessWindow?` :type Boolean))
  (return (and (<= (`KismetSystemLibrary.K2_GetTimerRemainingTimeHandle` (`self.Timer`)) 0.0) (<= (`KismetSystemLibrary.K2_GetTimerRemainingTimeHandle` (`self.Timer`)) (`self.SuccessWindow`)))))

(fn `StartAction`
  (if (`self.CanAttack`)
    (bind _returnvalue (`KismetSystemLibrary.K2_SetTimerDelegate` (`|CreateDelegate` :!event `ActionFinished`) (`self.Duration`)))
    (set `self.Timer` _returnvalue)
    (else
      (`KismetSystemLibrary.PrintString` "Cannot Attack yet!"))))