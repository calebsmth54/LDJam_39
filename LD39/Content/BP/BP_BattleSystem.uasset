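; Battle manager actor that runs one-on-one melee fights between the player and an enemy, with special music for the Villain boss.
; Battle start dims cached world lights and places a black void and spotlight between combatants; battle end reverses this.
; Tick checks for deaths and polls melee, attack and block windows to resolve hits, blocks and parries.
; Cooldown-finished events re-arm per-side damage flags, limiting damage to once per attack.
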(event `self.ReceiveBeginPlay`
  ;[1 1 1] Save all the world lights and their current intensity
  (`self.CacheWorldLights`))

(event `OnBattleStart`
  (params (Player :type "/Game/BP/Player/BP_PlayerCharacter Object Reference") (Enemy :type "/Game/BP/Enemies/BP_BaseEnemy Object Reference"))
  ;[1 1 1] Start Battle!
  (set `self.Player` Player)
  (set `self.Enemy` Enemy)
  ;[1 1 1] Setup environment for battle
  (`self.SetupForBattle`)
  ;[1 1 1] Limit player and enemy attacks to damage only once per attack cycle
  (add `/Game/BP/BP_Action.OnCoolDownFinished` (`/Game/BP/Player/BP_PlayerCharacter.MeleeAction` (`self.Player`)) (delegate `RefreshAttack`))
  (add `/Game/BP/BP_Action.OnCoolDownFinished` (`/Game/BP/Enemies/BP_BaseEnemy.AttackAction` (`self.Enemy`)) (delegate `EnemyCanAttackAgain`))
  ;[1 1 1] Set Battle States
  (set `self.InBattle` true)
  (set `self.CanPlayerDamage` true)
  (set `self.CanEnemyDamage` true)
  (cast `/Game/BP/Enemies/Villain` (`self.Enemy`) ; Check if the enemy is the final boss
    (:`then`
      ;[1 1 1] Play Finale Music
      (`/Game/BP/Player/BP_PlayerCharacter.PlayMusic` (`self.Player`) "/Game/Audio/Music/I_m_Sad_Cue.I_m_Sad_Cue"))
    (:`CastFailed`
      ;[1 1 1] Start Battle Music
      (`/Game/BP/Player/BP_PlayerCharacter.PlayMusic` (`self.Player`) "/Game/Audio/Music/Battle_-_Actions_Make_Music_Cue.Battle_-_Actions_Make_Music_Cue"))))

(event `RefreshAttack`
  ;[1 1 1] Limit player and enemy attacks to damage only once per attack cycle
  (set `self.CanPlayerDamage` true))

(event `EnemyCanAttackAgain`
  ;[1 1 1] Limit player and enemy attacks to damage only once per attack cycle
  (set `self.CanEnemyDamage` true))

(event `self.ReceiveTick`
  (params (DeltaSeconds :type "Float (single-precision)"))
  ;[1 1 1] Event Tick
  ;[1 1 1] Are we battling?
  (if (`self.InBattle`)
    ;[1 1 1] Is the player or the enemy dead?
    (if (`/Game/BP/BP_Health.IsDead?` (`/Game/BP/Player/BP_PlayerCharacter.Health` (`self.Player`)))
      ;[1 1 1] Play player death sound
      (`GameplayStatics.PlaySound2D` "/Game/Audio/SFX/Death.Death")
      ;[1 1 1] End Battle
      (set `self.InBattle` false :!label _label)
      (`self.EndBattle`)
      (elif (`/Game/BP/BP_Health.IsDead?` (`/Game/BP/Enemies/BP_BaseEnemy.Health` (`self.Enemy`)))
        ;[1 1 1] Play Enemy death sounds
        (`GameplayStatics.PlaySound2D` "/Game/Audio/SFX/Dead_Snake.Dead_Snake")
        (`GameplayStatics.PlaySound2D` "/Game/Audio/SFX/Hero_Beam_Cue.Hero_Beam_Cue")
        (goto _label)
        (else
          ;[1 1 1] Handle Melee Attacks
          (`self.HandleMeleeAttacks`))))))

(fn `CacheWorldLights`
  ;[1 1 1] Get All light actions so we can dim!
  (bind _outactors (`GameplayStatics.GetAllActorsOfClass` "/Script/Engine.Light"))
  (bind _output_get (set `self.WorldLightsArray` _outactors))
  ;[1 1 1] Save light intensities
  (for _array_element _output_get
    (`KismetArrayLibrary.Array_Add` (`self.WorldLightsIntensity`) (`LightComponentBase.Intensity` (`Light.LightComponent` _array_element)))))

(fn `DimWorldLights`
  ;[1 1 1] Dim all lights in the level
  (for _array_element (`self.WorldLightsArray`)
    (bind _lightcomponent (`Light.LightComponent` _array_element))
    (`LightComponent.SetIntensity` _lightcomponent (* (`LightComponentBase.Intensity` _lightcomponent) 0.25))))

(fn `EndBattle`
  ;[1 1 1] Let the enemy know combat has ended
  (`/Game/BP/Enemies/BP_BaseEnemy.OnCombatEnd` (`self.Enemy`))
  ;[1 1 1] Return world lights to normal
  (`self.UndimWorldLights`)
  ;[1 1 1] DeSpawn void
  (`SceneComponent.SetVisibility` (`self.BlackVoid`) false false)
  ;[1 1 1] Add Battle Spotlight
  (`SceneComponent.SetHiddenInGame` (`self.SpotLight`) true true)
  ;[1 1 1] Notify the player the combat has ended
  (`/Game/BP/Player/BP_PlayerCharacter.OnCombatEnd` (`self.Player`))
  ;[1 1 1] Unbind events so we can take on another player and enemy
  (clear `/Game/BP/BP_Action.OnCoolDownFinished` (`/Game/BP/Player/BP_PlayerCharacter.MeleeAction` (`self.Player`)))
  (clear `/Game/BP/BP_Action.OnCoolDownFinished` (`/Game/BP/Enemies/BP_BaseEnemy.AttackAction` (`self.Enemy`)))
  ;[1 1 1] Stop Battle Music
  (`/Game/BP/Player/BP_PlayerCharacter.StopMusic` (`self.Player`)))

(fn `HandleMeleeAttacks`
  ;[1 1 1] Is the player melee attacking?
  (if (`/Game/BP/BP_Action.IsInWindow` (`/Game/BP/Player/BP_PlayerCharacter.MeleeAction` (`self.Player`)))
    ;[1 1 1] Is the enemy attacking?
    (if (`/Game/BP/BP_Action.IsInWindow` (`/Game/BP/Enemies/BP_BaseEnemy.AttackAction` (`self.Enemy`)))
      ;[1 1 1] Can Damage be dealt?
      (if (and (`self.CanPlayerDamage`) (`self.CanEnemyDamage`))
        ;[1 1 1] Parry
        (`KismetSystemLibrary.PrintString` "Parry!")
        (`self.HandleParry`))
      (elif (`self.CanPlayerDamage`)
        ;[1 1 1] Dispense Damage to enemy
        (`/Game/BP/BP_Health.TakeDamage` (`/Game/BP/Enemies/BP_BaseEnemy.Health` (`self.Enemy`)) false)
        (set `self.CanPlayerDamage` false)
        ;[1 1 1] Enemy Sound
        (switch `int` (`KismetMathLibrary.RandomInteger` 2)
          (:`0`
            (`GameplayStatics.PlaySound2D` "/Game/Audio/SFX/lizard_hurt.lizard_hurt"))
          (:`1`
            (`GameplayStatics.PlaySound2D` "/Game/Audio/SFX/lizard_hurt1.lizard_hurt1")))))
    (else
      ;[1 1 1] Is the enemy attacking?
      (if (`/Game/BP/BP_Action.IsInWindow` (`/Game/BP/Enemies/BP_BaseEnemy.AttackAction` (`self.Enemy`)))
        ;[1 1 1] Is the player blocking?
        (if (`/Game/BP/BP_Action.IsInWindow` (`/Game/BP/Player/BP_PlayerCharacter.BlockAction` (`self.Player`)))
          (if (`self.CanEnemyDamage`)
            ;[1 1 1] Blocked!
            (`KismetSystemLibrary.PrintString` "BLOCKED!")
            (set `self.CanEnemyDamage` false)
            ;[1 1 1] PlayerSound
            (`GameplayStatics.PlaySound2D` "/Game/Audio/SFX/Hero_Block_Cue.Hero_Block_Cue"))
          (elif (`self.CanEnemyDamage`)
            ;[1 1 1] Dispense damge to player
            (`/Game/BP/BP_Health.TakeDamage` (`/Game/BP/Player/BP_PlayerCharacter.Health` (`self.Player`)) false)
            (set `self.CanEnemyDamage` false)
            ;[1 1 1] Player Sound
            (switch `int` (`KismetMathLibrary.RandomInteger` 2)
              (:`Default`
                (`GameplayStatics.PlaySound2D` "/Game/Audio/SFX/HURT_1.HURT_1" :!label _label))
              (:`0`
                (goto _label))
              (:`1`
                (`GameplayStatics.PlaySound2D` "/Game/Audio/SFX/HURT_2.HURT_2")))))
        (else
          ;[1 1 1] Nothing!
          (if true
            _))))))

(fn `HandleParry`
  ;[1 1 1] Handle Parry
  (set `self.CanPlayerDamage` false)
  (set `self.CanEnemyDamage` false)
  (`/Game/BP/Player/BP_PlayerCharacter.OnParry` (`self.Player`))
  (`/Game/BP/Enemies/BP_BaseEnemy.OnParry` (`self.Enemy`))
  (`GameplayStatics.PlaySound2D` "/Game/Audio/SFX/Hero_Block_Cue.Hero_Block_Cue")
  (`GameplayStatics.PlaySound2D` "/Game/Audio/SFX/Lizard_Defend.Lizard_Defend"))

(fn `SetupForBattle`
  (`self.DimWorldLights`)
  (bind _returnvalue (`self.SpawnBattleBackground`))
  (`self.ShowSpotlight` _returnvalue))

(fn `ShowSpotlight`
  (params (CenterOfArena :type "Vector Structure"))
  (bind _spotlight (`self.SpotLight`))
  ;[1 1 1] Add Battle Spotlight
  (`SceneComponent.K2_SetWorldLocation` _spotlight (+ (0.0 0.0 300.0) CenterOfArena) false false)
  (`SceneComponent.SetHiddenInGame` _spotlight false false))

(fn `SpawnBattleBackground`
  (returns (ReturnValue :type "Vector Structure"))
  (bind _returnvalue (`self.K2_GetActorLocation` (`self.Enemy`)))
  (bind _returnvalue_2 (+ (* (- (`self.K2_GetActorLocation` (`self.Player`)) _returnvalue) 0.5) _returnvalue))
  ;[1 1 1] Spawn void
  (`SceneComponent.K2_SetWorldLocation` (`self.BlackVoid`) (+ (0.0 0.0 -120.0) _returnvalue_2) false false)
  (`SceneComponent.SetVisibility` (`self.BlackVoid`) true true)
  (return _returnvalue_2))

(fn `UndimWorldLights`
  ;[1 1 1] Return lights to normal
  (for (_array_element _array_index) (`self.WorldLightsArray`)
    (`LightComponent.SetIntensity` (`Light.LightComponent` _array_element) (`|GetArrayItem` (`self.WorldLightsIntensity`) _array_index))))

(fn `UserConstructionScript`)