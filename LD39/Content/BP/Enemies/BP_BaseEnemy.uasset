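; Base enemy Blueprint that runs simple combat AI by picking weighted random actions from idle and attack.
; Overlapping CombatTrigger with the player notifies them of combat, turns the enemy to face them and resets its action state.
; While alive and in combat, Tick rolls against cumulative ChanceOfActions whenever no action is active.
; Started actions block new decisions and bind finish and cooldown callbacks; OnParry and ActionFinished are empty.
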(event `self.ReceiveBeginPlay`
  (`self.SetupActions`))

(event `self.CombatTrigger.OnComponentBeginOverlap`
  (params (OverlappedComponent :type "PrimitiveComponent Object Reference") (OtherActor :type "Actor Object Reference") (OtherComp :type "PrimitiveComponent Object Reference") (OtherBodyIndex :type Integer) (bFromSweep :type Boolean) (SweepResult :type "HitResult Structure (by ref)"))
  ;[1 1 1] Start Combat
  (if (not (`/Game/BP/BP_Health.IsDead?` (`self.Health`)))
    (bind _asbp_player_character (cast `/Game/BP/Player/BP_PlayerCharacter` OtherActor))
    (bind _output_get (set `self.PlayerAttacker` _asbp_player_character))
    (`/Game/BP/Player/BP_PlayerCharacter.OnEnterCombat` _asbp_player_character self)
    (`/Game/BP/Player/BP_PlayerCharacter.OnEnterCombat` _output_get self)
    ;[1 1 1] Face Player
    (`self.K2_SetActorRotation` (`KismetMathLibrary.Conv_VectorToRotator` (- (`self.K2_GetActorLocation` (`self.PlayerAttacker`)) (`self.K2_GetActorLocation`))))
    (`self.ResetStates`)
    (set `self.InCombat` true)))

(event `self.ReceiveTick`
  (params (DeltaSeconds :type "Float (single-precision)"))
  ;[1 1 1] Think!
  (`self.BaseThink` DeltaSeconds))

(event `OnParry`)

(fn `ActionFinished`)

(fn `BaseThink`
  (params (Delta :type "Float (double-precision)"))
  ;[1 1 1] In Combat or dead?
  (if (and (`self.InCombat`) (not (`/Game/BP/BP_Health.IsDead?` (`self.Health`))))
    ;[1 1 1] Are we already acting?
    (if (not (`self.InActionState`))
      ;[1 1 1] Make a new decision!
      (bind _actionchosen (`self.ChooseRandomAction`))
      (bind _output_get (set `self.SelectedAction` _actionchosen))
      (`KismetSystemLibrary.PrintString` (`KismetStringLibrary.Concat_StrStr` "Chose Action: " (`KismetStringLibrary.Conv_IntToString` _output_get)))
      (`self.StartAction`))))

(fn `ChooseRandomAction`
  (returns (ActionChosen :type Integer))
  (locals (Accumulator :type "Float (double-precision)" :default 0.0) (RandomVal :type "Float (double-precision)"))
  (set `local.RandomVal` (`KismetMathLibrary.RandomFloat`))
  (set `local.Accumulator` 0.0)
  (for _index (range (+ (`KismetArrayLibrary.Array_Length` (`self.ChanceOfActions`)) 1))
    (set `local.Accumulator` (+ (`|GetArrayItem` (`self.ChanceOfActions`) _index) (`local.Accumulator`)))
    (if (<= (`local.RandomVal`) (`local.Accumulator`))
      (break)))
  (return _index))

(fn `ReadyToAct`
  (set `self.InActionState` false))

(fn `ResetStates`
  (set `self.InActionState` false))

(fn `SetupActions`
  (`KismetArrayLibrary.Array_Insert` (`self.ActionList`) (`self.IdleAction`))
  (`KismetArrayLibrary.Array_Insert` (`self.ActionList`) (`self.AttackAction`) 1))

(fn `StartAction`
  (bind _output (`|GetArrayItem` (`self.ActionList`) (`self.SelectedAction`)))
  (bind _success_ (`/Game/BP/BP_Action.StartAction` _output))
  (if _success_
    (add `/Game/BP/BP_Action.OnActionFished` _output (`|CreateDelegate` :!event `ActionFinished`))
    (add `/Game/BP/BP_Action.OnCoolDownFinished` _output (`|CreateDelegate` :!event `ReadyToAct`))
    (set `self.InActionState` true)))

(fn `UserConstructionScript`)