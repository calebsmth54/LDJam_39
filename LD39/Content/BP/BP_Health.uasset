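; BP_Health is a health Blueprint that applies damage through a single TakeDamage function.
; A Quake flag selects the heavier hit, while any other hit removes a smaller fixed amount from CurrentHealth.
; Only the Quake branch checks for depleted health, setting IsDead and calling CallOnDeath; ordinary damage never triggers death.
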(fn `TakeDamage`
  (params (`Quake?` :type Boolean))
  (if `Quake?`
    (set `self.CurrentHealth` (- (`self.CurrentHealth`) 3))
    (if (<= (`self.CurrentHealth`) 0)
      (set `self.IsDead?` true)
      (`self.OnDeath`))
    (else
      (set `self.CurrentHealth` (- (`self.CurrentHealth`) 1)))))